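; LaunchBauncelot is a launcher that pushes the BPBouncelotStef ball along world +X with a fixed velocity-change impulse.
; Overlapping its CollisionComponent caches the Bouncelot reference and applies the impulse immediately.
; The ShootBall event reapplies that impulse to the cached reference, with a validity check that guards nothing.
; Debug prints remain, and the player-character lookup and GetShootBouncelot check are disconnected.
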(event OnComponentBeginOverlap(CollisionComponent)
  (params (OverlappedComponent :type Primitive%20Component%20Object%20Reference) (OtherActor :type Actor%20Object%20Reference) (OtherComp :type Primitive%20Component%20Object%20Reference) (OtherBodyIndex :type Integer) (bFromSweep :type Boolean) (SweepResult :type Hit%20Result%20Structure%20%28by%20ref%29))
  (bind _asbpbouncelot_stef (Utilities|Casting|CastToBPBouncelotStef OtherActor))
  (Physics|AddImpulse (Variables|/Game/Bouncelot/StefanoStuff/BluePrints/Bouncelot/BPBouncelotStef.BPBouncelotStef_C|GetBall _asbpbouncelot_stef) "500.000000,0.000000,0.000000" "None" true)
  (Development|PrintString "add impulse"))

(event Custom|ShootBall
  (bind _as_bpbouncelot_stef (Variables|Default|GetAs%20BPBouncelot%20Stef))
  (Development|PrintString "Hello")
  (Utilities|IsValid _as_bpbouncelot_stef
    (:Is%20Valid
      _)
    (:Is%20Not%20Valid
      _))
  (Physics|AddImpulse (Variables|/Game/Bouncelot/StefanoStuff/BluePrints/Bouncelot/BPBouncelotStef.BPBouncelotStef_C|GetBall _as_bpbouncelot_stef) "500.000000,0.000000,0.000000" "None" true)
  (Development|PrintString "shooting"))

(fn ConstructionScript)