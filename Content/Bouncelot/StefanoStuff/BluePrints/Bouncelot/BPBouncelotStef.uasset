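; BPBouncelotStef is the Bouncelot ball pawn, which adds its Enhanced Input mapping on BeginPlay and handles dashing and pawn switching.
; Dash traces from the mouse cursor and pushes the Ball with a force derived from the hit's impact normal minus the ball actor's location.
; Shoot and flipper inputs make player 0 possess the stored launcher or flipper pawn.
; The launcher's cast and ShootBall logic is disconnected.
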(event Custom|PossessPawn
  (params (NewParam :type Default%20Pawn%20Object%20Reference))
  ;[0.008122 0.15 0.02347 0.5] Pawns possession
  (Pawn|Possess (Game|GetPlayerController 0) NewParam))

(event Input|EnhancedActionEvents|EnhancedInputActionShootBouncelot
  (params (ActionValue :type Boolean) (ElapsedSeconds :type Float%20%28double-precision%29) (TriggeredSeconds :type Float%20%28double-precision%29) (InputAction :type Input%20Action%20Object%20Reference :default "/Game/Bouncelot/StefanoStuff/Input/ShootBouncelot.ShootBouncelot"))
  ;[0.008122 0.15 0.02347 0.5] Pawns possession
  (:Started
    (CallFunction|PossessPawn (Variables|Default|GetAs%20Launch%20Bauncelot))))

(event Input|EnhancedActionEvents|EnhancedInputActionDash
  (params (ActionValue :type Boolean) (ElapsedSeconds :type Float%20%28double-precision%29) (TriggeredSeconds :type Float%20%28double-precision%29) (InputAction :type Input%20Action%20Object%20Reference :default "/Game/Bouncelot/StefanoStuff/Input/Dash.Dash"))
  ;[0.15 0 0.1089 0.5] Dash
  (bind _returnvalue (Class|WidgetLayoutLibrary|GetMousePositiononViewport))
  (bind _outhit (Collision|LineTraceByChannel (.WorldPosition (Class|GameplayStatics|DeprojectScreentoWorld (Game|GetPlayerController 0) (Math|Vector2D|MakeVector2D (.x _returnvalue) (.y _returnvalue)))) (* (+ (.WorldDirection (Class|GameplayStatics|DeprojectScreentoWorld (Game|GetPlayerController 0) (Math|Vector2D|MakeVector2D (.x _returnvalue) (.y _returnvalue)))) (.WorldPosition (Class|GameplayStatics|DeprojectScreentoWorld (Game|GetPlayerController 0) (Math|Vector2D|MakeVector2D (.x _returnvalue) (.y _returnvalue))))) 1e+09) "TraceTypeQuery1" false 0 "None"))
  (bind _returnvalue_2 (Actor|GetActorOfClass "BPBouncelotStef_C"))
  (Physics|AddForce (Variables|BPBouncelotStef_C|GetBall _returnvalue_2) (* (Math|Vector|Normalize (- (.ImpactNormal (Collision|BreakHitResult _outhit)) (Transformation|GetActorLocation _returnvalue_2))) 4.5e+04) "None" false)
  (Development|PrintString "dashing"))

(event Input|EnhancedActionEvents|EnhancedInputActionUseFlipperLeft
  (params (ActionValue :type Boolean) (ElapsedSeconds :type Float%20%28double-precision%29) (TriggeredSeconds :type Float%20%28double-precision%29) (InputAction :type Input%20Action%20Object%20Reference :default "/Game/Bouncelot/StefanoStuff/Input/UseFlipperLeft.UseFlipperLeft"))
  ;[0.008122 0.15 0.02347 0.5] Pawns possession
  (:Started
    (CallFunction|PossessPawn (Variables|Default|GetAs%20BPFlipper%20Left))))

(event Input|EnhancedActionEvents|EnhancedInputActionUseFlipperRight
  (params (ActionValue :type Boolean) (ElapsedSeconds :type Float%20%28double-precision%29) (TriggeredSeconds :type Float%20%28double-precision%29) (InputAction :type Input%20Action%20Object%20Reference :default "/Game/Bouncelot/StefanoStuff/Input/UseFlipperRight.UseFlipperRight"))
  ;[0.008122 0.15 0.02347 0.5] Pawns possession
  (:Started
    (CallFunction|PossessPawn (Variables|Default|GetAs%20BPFlipper%20Right))))

(event EventBeginPlay
  ;[0.000914 0.008428 0.15 0.5] Input Mapping
  (bind _asplayer_controller (Utilities|Casting|CastToPlayerController (Pawn|GetController)))
  (Utilities|IsValid (PlayerController|LocalPlayerSubsystems|GetEnhancedInputLocalPlayerSubsystem _asplayer_controller)
    (:Is%20Valid
      (Input|AddMappingContext (PlayerController|LocalPlayerSubsystems|GetEnhancedInputLocalPlayerSubsystem _asplayer_controller) "/Game/Bouncelot/StefanoStuff/Input/StefanoInputMapping.StefanoInputMapping" 0 "(bIgnoreAllPressedKeysUntilRelease=True,bForceImmediately=False,bNotifyUserSettings=False)")
      ;[0.1155 0.02984 0.15 0.5] Possess the pawns
      (bind _returnvalue (Actor|GetActorOfClass (Variables|Default|GetActor%20Class)))
      (Variables|Default|SetPawnPossessed _returnvalue))))

(fn ConstructionScript)