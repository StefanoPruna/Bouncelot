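; Bouncelot Blueprint that launches a physics Ball and handles a mouse-based dash input.
; ShootBouncelot input and the LaunchBall event share one fixed +X velocity-change impulse on Ball.
; Dash traces from the deprojected cursor, then applies force to the root of an actor found by class.
; The force direction is the normalized hit ImpactNormal minus that actor's location, so it uses the surface normal rather than the hit point.
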(event Custom|LaunchBall
  (Physics|AddImpulse (Variables|Default|GetBall) "1000.000000,0.000000,0.000000" "None" true))

(event Input|EnhancedActionEvents|EnhancedInputActionDash
  (params (ActionValue :type Boolean) (ElapsedSeconds :type Float%20%28double-precision%29) (TriggeredSeconds :type Float%20%28double-precision%29) (InputAction :type Input%20Action%20Object%20Reference :default "/Game/Bouncelot/StefanoStuff/Input/Dash.Dash"))
  ;[0.15 0 0.1089 0.5] Dash
  (bind _returnvalue (Class|WidgetLayoutLibrary|GetMousePositiononViewport))
  (bind _outhit (Collision|LineTraceByChannel (.WorldPosition (Class|GameplayStatics|DeprojectScreentoWorld (Game|GetPlayerController 0) (Math|Vector2D|MakeVector2D (.x _returnvalue) (.y _returnvalue)))) (* (+ (.WorldDirection (Class|GameplayStatics|DeprojectScreentoWorld (Game|GetPlayerController 0) (Math|Vector2D|MakeVector2D (.x _returnvalue) (.y _returnvalue)))) (.WorldPosition (Class|GameplayStatics|DeprojectScreentoWorld (Game|GetPlayerController 0) (Math|Vector2D|MakeVector2D (.x _returnvalue) (.y _returnvalue))))) 1e+09) "TraceTypeQuery1" false 0 "None"))
  (bind _returnvalue_2 (Actor|GetActorOfClass 0))
  (bind _asprimitive_component (Utilities|Casting|CastToPrimitiveComponent (Variables|/Script/Engine.Actor|GetRootComponent _returnvalue_2)))
  (Physics|AddForce _asprimitive_component (* (Math|Vector|Normalize (- (.ImpactNormal (Collision|BreakHitResult _outhit)) (Transformation|GetActorLocation _returnvalue_2))) 4.5e+04) "None" false))

(event Input|EnhancedActionEvents|EnhancedInputActionShootBouncelot
  (params (ActionValue :type Boolean) (ElapsedSeconds :type Float%20%28double-precision%29) (TriggeredSeconds :type Float%20%28double-precision%29) (InputAction :type Input%20Action%20Object%20Reference :default "/Game/Bouncelot/StefanoStuff/Input/ShootBouncelot.ShootBouncelot"))
  (Physics|AddImpulse (Variables|Default|GetBall) "1000.000000,0.000000,0.000000" "None" true))

(event EventBeginPlay)

(event Input|KeyboardEvents|F
  (params (Key :type Key%20Structure :default "None")))

(fn ConstructionScript)