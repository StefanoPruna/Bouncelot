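; BPFlipper is a pair of pinball-style flippers that the player triggers to knock the BPBouncelot ball.
; Enhanced Input starts a separate timeline per paddle, which lerps its relative yaw, pauses briefly, then reverses.
; Overlapping either paddle's collision calls Push, which applies a fixed +X impulse to the ball's sphere, regardless of whether the flipper is moving.
; Velocity-based repulsion and IsActive gating are left disconnected.
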(event OnComponentBeginOverlap(PaddleCollisionLeft)
  (params (OverlappedComponent :type Primitive%20Component%20Object%20Reference) (OtherActor :type Actor%20Object%20Reference) (OtherComp :type Primitive%20Component%20Object%20Reference) (OtherBodyIndex :type Integer) (bFromSweep :type Boolean) (SweepResult :type Hit%20Result%20Structure%20%28by%20ref%29))
  ;[0.01904 0.03165 0.15 0.5] Flippers push the ball
  (CallFunction|Push OtherActor))

(event OnComponentBeginOverlap(PaddleCollisionRight)
  (params (OverlappedComponent :type Primitive%20Component%20Object%20Reference) (OtherActor :type Actor%20Object%20Reference) (OtherComp :type Primitive%20Component%20Object%20Reference) (OtherBodyIndex :type Integer) (bFromSweep :type Boolean) (SweepResult :type Hit%20Result%20Structure%20%28by%20ref%29))
  ;[0.01904 0.03165 0.15 0.5] Flippers push the ball
  (CallFunction|Push OtherActor))

(event OnComponentHit(PaddleCollisionLeft)
  (params (HitComponent :type Primitive%20Component%20Object%20Reference) (OtherActor :type Actor%20Object%20Reference) (OtherComp :type Primitive%20Component%20Object%20Reference) (NormalImpulse :type Vector :default "0, 0, 0") (Hit :type Hit%20Result%20Structure%20%28by%20ref%29)))

(event Custom|Push
  (params (OtherActor :type Actor%20Object%20Reference))
  ;[0.01904 0.03165 0.15 0.5] Flippers push the ball
  (if true
    (bind _asbpbouncelot (Utilities|Casting|CastToBPBouncelot OtherActor))
    (Physics|AddImpulse (Variables|/Game/Bouncelot/StefanoStuff/BluePrints/Bouncelot/BPBouncelot.BPBouncelot_C|GetSphere _asbpbouncelot) "2000.000000,0.000000,0.000000" "None" false)))

(event Input|EnhancedActionEvents|EnhancedInputActionUseFlipperLeft
  (params (ActionValue :type Boolean) (ElapsedSeconds :type Float%20%28double-precision%29) (TriggeredSeconds :type Float%20%28double-precision%29) (InputAction :type Input%20Action%20Object%20Reference :default "/Game/Bouncelot/StefanoStuff/Input/UseFlipperLeft.UseFlipperLeft"))
  ;[0.02859 0.15 0.0113 0.5] Flippers' movement
  (:Started
    (bind _left (Timeline|LeftFlipper Play)
      (:Update
        (Transformation|SetRelativeRotation (Variables|Default|GetLeftPaddle) (Math|Rotator|MakeRotator 0.0 0.0 (Math|Float|Lerp 2e+01 -44.0 _left)) false false))
      (:Finished
        (Utilities|FlowControl|Delay 0.5)
        (Timeline|LeftFlipper Reverse)))))

(event Input|EnhancedActionEvents|EnhancedInputActionUseFlipperRight
  (params (ActionValue :type Boolean) (ElapsedSeconds :type Float%20%28double-precision%29) (TriggeredSeconds :type Float%20%28double-precision%29) (InputAction :type Input%20Action%20Object%20Reference :default "/Game/Bouncelot/StefanoStuff/Input/UseFlipperRight.UseFlipperRight"))
  ;[0.02859 0.15 0.0113 0.5] Flippers' movement
  (:Started
    (bind _right (Timeline|Right PlayFromStart)
      (:Update
        (Transformation|SetRelativeRotation (Variables|Default|GetRightPaddle) (Math|Rotator|MakeRotator 0.0 0.0 (Math|Float|Lerp -195.0 -1.5e+02 _right)) false false))
      (:Finished
        (Utilities|FlowControl|Delay 0.7)
        (Timeline|Right Reverse)))))

(event EventBeginPlay
  (bind _returnvalue (Game|GetPlayerController 0))
  (bind _returnvalue_2 (PlayerController|LocalPlayerSubsystems|GetEnhancedInputLocalPlayerSubsystem _returnvalue))
  ;[0.000914 0.008428 0.15 0.5] Input Mapping
  (Utilities|IsValid _returnvalue_2
    (:Is%20Valid
      (Input|AddMappingContext _returnvalue_2 "/Game/Bouncelot/StefanoStuff/Input/StefanoInputMapping.StefanoInputMapping" 0 "(bIgnoreAllPressedKeysUntilRelease=True,bForceImmediately=False,bNotifyUserSettings=False)"))))

(fn ConstructionScript)